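; BP_CAmreaSystem is a shared camera actor for two players that becomes player 0's view target at BeginPlay.
; Each tick it moves to the midpoint between both characters and prints that vector's length.
; Past a threshold, field of view scales with that length, which measures distance from world origin rather than player separation.
; Within a band above the threshold, it reasserts itself as view target for both controllers.
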(event EventBeginPlay
  ;[1 0.7647 0] setting players to vars
  (Variables|Default|SetPlayer1 (Game|GetPlayerCharacter 0))
  (Variables|Default|SetPlayer2 (Game|GetPlayerCharacter 1))
  ;[1 0.7647 0] Setting Camera As active camera
  (Game|Player|SetViewTargetwithBlend (Game|GetPlayerController 0) self 0.0 "VTBlend_Linear" 0.0 false))

(event EventTick
  (params (DeltaSeconds :type Float%20%28single-precision%29))
  (bind _player1 (Variables|Default|GetPlayer1))
  (bind _player2 (Variables|Default|GetPlayer2))
  (bind _returnvalue (Transformation|GetActorTransform _player2))
  (bind _returnvalue_2 (Transformation|GetActorTransform _player1))
  ;[1 0.7647 0] Assiginig Camera to MidPointLocation
  (bind _output_get (Variables|Default|SetMidPointVector (Math|Vector|MakeVector (/ (+ (.x (.location _returnvalue_2)) (.x (.location _returnvalue))) 2.0) (/ (+ (.y (.location _returnvalue_2)) (.y (.location _returnvalue))) 2.0) (/ (+ (.z (.location _returnvalue_2)) (.z (.location _returnvalue))) 2.0))))
  (Transformation|SetActorLocation (Variables|Default|GetMidPointVector) false false)
  (Development|PrintString (Utilities|String|ToString(Float) (Math|Vector|VectorLength _output_get)))
  (if (> (Math|Vector|VectorLength _output_get) 7e+02)
    (Camera|SetFieldOfView (Variables|Default|GetCamera) (* (/ (Math|Vector|VectorLength _output_get) 7e+02) 9e+01))
    (if (not (> (Math|Vector|VectorLength _output_get) 9e+02))
      (if (< (Math|Vector|VectorLength _output_get) 9e+02)
        (Game|Player|SetViewTargetwithBlend (Game|GetPlayerController 0) self 0.0 "VTBlend_Linear" 0.0 false)))))

(fn ConstructionScript)