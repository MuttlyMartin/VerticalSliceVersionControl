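; Boulder crane obstacle that launches and temporarily ragdolls the player character when its sphere is hit.
; A timeline, played from Tick, rotates the cube by interpolating its relative rotation through 120 degrees on one axis.
; Sphere overlap applies a fixed launch velocity to BP_Character1, briefly waits, then enables ragdoll and Flying movement before calling TurnOffRagDoll after another delay.
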(event OnComponentBeginOverlap(Sphere)
  (params (OverlappedComponent :type Primitive%20Component%20Object%20Reference) (OtherActor :type Actor%20Object%20Reference) (OtherComp :type Primitive%20Component%20Object%20Reference) (OtherBodyIndex :type Integer) (bFromSweep :type Boolean) (SweepResult :type Hit%20Result%20Structure%20%28by%20ref%29))
  (bind _asbp_character_1 (Utilities|Casting|CastToBP_Character1 OtherActor))
  (bind _ascharacter (Utilities|Casting|CastToCharacter OtherActor))
  (Character|LaunchCharacter _ascharacter "1250.000000,-1000.000000,1250.000000" false false)
  (Utilities|FlowControl|Delay 0.2)
  (Variables|/Game/Dynamic/CharacterFiles/CharacterBP/BP_Character1.BP_Character1_C|SetRagdoll _asbp_character_1 true)
  (Pawn|Components|CharacterMovement|SetMovementMode (Variables|/Script/Engine.Character|GetCharacterMovement _asbp_character_1) "MOVE_Flying" 0)
  (Utilities|FlowControl|Delay 2.0)
  (Default|TurnOffRagDoll _asbp_character_1))

(event EventTick
  (params (DeltaSeconds :type Float%20%28single-precision%29))
  (bind _rotating (Timeline|Rotating Play)
    (:Update
      (Transformation|SetRelativeRotation (Variables|Default|GetCube) (Math|Rotator|Lerp(Rotator) "0, 0, 0" "0.000000,120.000000,0.000000" _rotating) false false))))

(fn ConstructionScript)