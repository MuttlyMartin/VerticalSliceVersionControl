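; BP_BuzzSaw is a spinning saw hazard that knocks player characters away on contact.
; Tick plays the Spin timeline, which lerps the blade mesh's relative yaw through a full turn.
; Box overlap casts to BP_Character1 or BP_Character2, adds a fixed launch velocity regardless of approach direction, and ragdolls the victim briefly before restoring it.
; The two character classes use duplicated but identical branches.
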(event OnComponentBeginOverlap(Box)
  (params (OverlappedComponent :type Primitive%20Component%20Object%20Reference) (OtherActor :type Actor%20Object%20Reference) (OtherComp :type Primitive%20Component%20Object%20Reference) (OtherBodyIndex :type Integer) (bFromSweep :type Boolean) (SweepResult :type Hit%20Result%20Structure%20%28by%20ref%29))
  (bind _asbp_character_1 (Utilities|Casting|CastToBP_Character1 OtherActor)
    (:then
      (bind _ascharacter (Utilities|Casting|CastToCharacter OtherActor))
      (Character|LaunchCharacter _ascharacter "1250.000000,-1000.000000,1250.000000" false false)
      (Default|ActivateRagdoll _asbp_character_1)
      (Utilities|FlowControl|Delay 1.0)
      (Default|TurnOffRagDoll _asbp_character_1))
    (:CastFailed
      (bind _asbp_character_2 (Utilities|Casting|CastToBP_Character2 OtherActor))
      (bind _ascharacter_2 (Utilities|Casting|CastToCharacter OtherActor))
      (Character|LaunchCharacter _ascharacter_2 "1250.000000,-1000.000000,1250.000000" false false)
      (Default|ActivateRagdoll _asbp_character_2)
      (Utilities|FlowControl|Delay 1.0)
      (Default|TurnOffRagDoll _asbp_character_2))))

(event EventTick
  (params (DeltaSeconds :type Float%20%28single-precision%29))
  (bind _spinning (Timeline|spin Play)
    (:Update
      (Transformation|SetRelativeRotation (Variables|Default|GetBuzzSaw_pCylinder1) (Math|Rotator|Lerp(Rotator) "0, 0, 0" "-360.000000,0.000000,0.000000" _spinning) false false))))

(fn ConstructionScript)