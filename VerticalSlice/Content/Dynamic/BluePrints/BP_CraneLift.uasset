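; BP_CraneLift is a crane lift actor that raises and lowers a Crate component using two overlap triggers.
; The GoingUp timeline drives a lerp of the crate's relative location between DownPos and UpPos.
; Overlapping UpCol plays the timeline, DownCol reverses it, and leaving either trigger stops the crate in place.
; The IsUp and GoingDown nodes are disconnected and never run.
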(event OnComponentBeginOverlap(DownCol)
  (params (OverlappedComponent :type Primitive%20Component%20Object%20Reference) (OtherActor :type Actor%20Object%20Reference) (OtherComp :type Primitive%20Component%20Object%20Reference) (OtherBodyIndex :type Integer) (bFromSweep :type Boolean) (SweepResult :type Hit%20Result%20Structure%20%28by%20ref%29))
  (bind _goingup (Timeline|GoingUp Reverse)
    (:Update
      (Transformation|SetRelativeLocation (Variables|Default|GetCrate) (Math|Vector|Lerp(Vector) (Variables|Default|GetDownPos) (Variables|Default|GetUpPos) _goingup) false false))))

(event OnComponentBeginOverlap(UpCol)
  (params (OverlappedComponent :type Primitive%20Component%20Object%20Reference) (OtherActor :type Actor%20Object%20Reference) (OtherComp :type Primitive%20Component%20Object%20Reference) (OtherBodyIndex :type Integer) (bFromSweep :type Boolean) (SweepResult :type Hit%20Result%20Structure%20%28by%20ref%29))
  (bind _goingup (Timeline|GoingUp Play)
    (:Update
      (Transformation|SetRelativeLocation (Variables|Default|GetCrate) (Math|Vector|Lerp(Vector) (Variables|Default|GetDownPos) (Variables|Default|GetUpPos) _goingup) false false))))

(event OnComponentEndOverlap(DownCol)
  (params (OverlappedComponent :type Primitive%20Component%20Object%20Reference) (OtherActor :type Actor%20Object%20Reference) (OtherComp :type Primitive%20Component%20Object%20Reference) (OtherBodyIndex :type Integer))
  (bind _goingup (Timeline|GoingUp Stop)
    (:Update
      (Transformation|SetRelativeLocation (Variables|Default|GetCrate) (Math|Vector|Lerp(Vector) (Variables|Default|GetDownPos) (Variables|Default|GetUpPos) _goingup) false false))))

(event OnComponentEndOverlap(UpCol)
  (params (OverlappedComponent :type Primitive%20Component%20Object%20Reference) (OtherActor :type Actor%20Object%20Reference) (OtherComp :type Primitive%20Component%20Object%20Reference) (OtherBodyIndex :type Integer))
  (bind _goingup (Timeline|GoingUp Stop)
    (:Update
      (Transformation|SetRelativeLocation (Variables|Default|GetCrate) (Math|Vector|Lerp(Vector) (Variables|Default|GetDownPos) (Variables|Default|GetUpPos) _goingup) false false))))

(fn ConstructionScript)