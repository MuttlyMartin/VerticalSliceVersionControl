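; Elevator actor with sliding doors that can break and drop down its shaft onto an enemy placed at the bottom.
; Timelines lerp the enemy to the shaft end on BeginPlay, drop the elevator on EvevatorBreaks, and open or close doors on entry and exit trigger overlaps.
; Tick compares elevator and enemy locations to call KillMonster, which is empty here.
; A text trigger prints a kill message or hint from the same comparison.
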(event OnComponentBeginOverlap(EnterBox)
  (params (OverlappedComponent :type Primitive%20Component%20Object%20Reference) (OtherActor :type Actor%20Object%20Reference) (OtherComp :type Primitive%20Component%20Object%20Reference) (OtherBodyIndex :type Integer) (bFromSweep :type Boolean) (SweepResult :type Hit%20Result%20Structure%20%28by%20ref%29))
  ;[1 0.8529 0] Open/Close elevator
  (bind _opening_closing (Timeline|Opening/Closing Play)
    (:Update
      (Transformation|SetRelativeLocation (Variables|Default|GetLeftDoor) (Math|Vector|Lerp(Vector) (Variables|Default|GetLeftDoorA) (Variables|Default|GetLeftDoorB) _opening_closing) false false)
      (Transformation|SetRelativeLocation (Variables|Default|GetRightDoor) (Math|Vector|Lerp(Vector) (Variables|Default|GetRightDoorA) (Variables|Default|GetRightDoorB) _opening_closing) false false))))

(event OnComponentBeginOverlap(ExsitBox)
  (params (OverlappedComponent :type Primitive%20Component%20Object%20Reference) (OtherActor :type Actor%20Object%20Reference) (OtherComp :type Primitive%20Component%20Object%20Reference) (OtherBodyIndex :type Integer) (bFromSweep :type Boolean) (SweepResult :type Hit%20Result%20Structure%20%28by%20ref%29))
  ;[1 0.8529 0] Open/Close elevator
  (bind _opening_closing (Timeline|Opening/Closing Play)
    (:Update
      (Transformation|SetRelativeLocation (Variables|Default|GetLeftDoor) (Math|Vector|Lerp(Vector) (Variables|Default|GetLeftDoorA) (Variables|Default|GetLeftDoorB) _opening_closing) false false)
      (Transformation|SetRelativeLocation (Variables|Default|GetRightDoor) (Math|Vector|Lerp(Vector) (Variables|Default|GetRightDoorA) (Variables|Default|GetRightDoorB) _opening_closing) false false))))

(event OnComponentEndOverlap(EnterBox)
  (params (OverlappedComponent :type Primitive%20Component%20Object%20Reference) (OtherActor :type Actor%20Object%20Reference) (OtherComp :type Primitive%20Component%20Object%20Reference) (OtherBodyIndex :type Integer))
  ;[1 0.8529 0] Open/Close elevator
  (bind _opening_closing (Timeline|Opening/Closing Reverse)
    (:Update
      (Transformation|SetRelativeLocation (Variables|Default|GetLeftDoor) (Math|Vector|Lerp(Vector) (Variables|Default|GetLeftDoorA) (Variables|Default|GetLeftDoorB) _opening_closing) false false)
      (Transformation|SetRelativeLocation (Variables|Default|GetRightDoor) (Math|Vector|Lerp(Vector) (Variables|Default|GetRightDoorA) (Variables|Default|GetRightDoorB) _opening_closing) false false))))

(event OnComponentEndOverlap(ExsitBox)
  (params (OverlappedComponent :type Primitive%20Component%20Object%20Reference) (OtherActor :type Actor%20Object%20Reference) (OtherComp :type Primitive%20Component%20Object%20Reference) (OtherBodyIndex :type Integer))
  ;[1 0.8529 0] Open/Close elevator
  (bind _opening_closing (Timeline|Opening/Closing Reverse)
    (:Update
      (Transformation|SetRelativeLocation (Variables|Default|GetLeftDoor) (Math|Vector|Lerp(Vector) (Variables|Default|GetLeftDoorA) (Variables|Default|GetLeftDoorB) _opening_closing) false false)
      (Transformation|SetRelativeLocation (Variables|Default|GetRightDoor) (Math|Vector|Lerp(Vector) (Variables|Default|GetRightDoorA) (Variables|Default|GetRightDoorB) _opening_closing) false false))))

(event OnComponentBeginOverlap(TextFeild)
  (params (OverlappedComponent :type Primitive%20Component%20Object%20Reference) (OtherActor :type Actor%20Object%20Reference) (OtherComp :type Primitive%20Component%20Object%20Reference) (OtherBodyIndex :type Integer) (bFromSweep :type Boolean) (SweepResult :type Hit%20Result%20Structure%20%28by%20ref%29))
  ;[0.9957 1 0] ShowText
  (if (Utilities|Operators|EqualEqual (Variables|/Script/Engine.SceneComponent|GetRelativeLocation (Variables|Default|GetBoolean_B1AA06D2)) (Variables|/Script/Engine.SceneComponent|GetRelativeLocation (Variables|Default|Geteneime)) 0.0)
    (Development|PrintString "Weldone you killed iy!")
    (else
      (Development|PrintString "you something heavy to kill this one"))))

(event Custom|EvevatorBreaks
  (bind _boolean_b1aa06d2 (Variables|Default|GetBoolean_B1AA06D2))
  ;[1 0.9338 0] DropElevator
  (bind _newtrack_0 (Timeline|Drop Play)
    (:Update
      (Transformation|SetRelativeLocation _boolean_b1aa06d2 (Math|Vector|Lerp(Vector) (Variables|/Script/Engine.SceneComponent|GetRelativeLocation _boolean_b1aa06d2) (Variables|Default|GetShaftLength) _newtrack_0) false false))))

(event Custom|KillMonster)

(event EventTick
  (params (DeltaSeconds :type Float%20%28single-precision%29))
  ;[1 0.857 0] Checking if Dropped
  (if (Utilities|Operators|EqualEqual (Variables|/Script/Engine.SceneComponent|GetRelativeLocation (Variables|Default|GetBoolean_B1AA06D2)) (Variables|/Script/Engine.SceneComponent|GetRelativeLocation (Variables|Default|Geteneime)) 0.0)
    (CallFunction|KillMonster)))

(event EventBeginPlay
  ;[1 0.8772 0] sets location of enemy
  (bind _shaftlengthtimeline (Timeline|ShaftLengthTimeline Play)
    (:Update
      (Transformation|SetRelativeLocation (Variables|Default|Geteneime) (Math|Vector|Lerp(Vector) (Variables|/Script/Engine.SceneComponent|GetRelativeLocation (Variables|Default|Geteneime)) (Variables|Default|GetShaftLength) _shaftlengthtimeline) false false))))

(fn ConstructionScript)