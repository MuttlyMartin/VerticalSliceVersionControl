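; Enemy Blueprint actor with a health value and a widget component showing a healthbar.
; On BeginPlay it caches the Healthbar_W widget reference from the component.
; TakeDamage lowers Health by one and writes it into the widget's Health.
; Tick destroys the actor once Health reaches zero; the Updatehealth function is empty.
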(event Custom|TakeDamage
  (bind _output_get (Variables|Default|SetHealth (- (Variables|Default|GetHealth) 1)))
  (Variables|/Game/Dynamic/BluePrints/Healthbar_W.Healthbar_W_C|SetHealth (Variables|Default|GetHealthWidgetReference) (Math|Conversions|ToFloat(Integer) _output_get))
  (Utilities|FlowControl|Delay 0.2))

(event EventBeginPlay
  (bind _ashealthbar_w (Utilities|Casting|CastToHealthbar_W (UserInterface|GetUserWidgetObject (Variables|Default|GetWidget))))
  (bind _output_get (Variables|Default|SetHealthWidgetReference _ashealthbar_w)))

(event Collision|EventActorBeginOverlap
  (params (OtherActor :type Actor%20Object%20Reference)))

(event EventTick
  (params (DeltaSeconds :type Float%20%28single-precision%29))
  (if (<= (Variables|Default|GetHealth) 0)
    (Actor|DestroyActor)))

(fn ConstructionScript)

(fn Updatehealth)