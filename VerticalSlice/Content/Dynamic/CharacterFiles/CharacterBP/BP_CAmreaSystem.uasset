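; BP_CAmreaSystem is a shared camera actor that follows two player characters.
; BeginPlay caches players 0 and 1 and makes itself the first controller's view target.
; Each Tick averages both locations and moves the actor to that midpoint, without sweep.
; An unconnected branch would scale field of view by the midpoint vector's length (distance from world origin, not player separation), but it never runs.
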(event EventBeginPlay
  ;[1 0.7647 0] setting players to vars
  (Variables|Default|SetPlayer1 (Game|GetPlayerCharacter 0))
  (Variables|Default|SetPlayer2 (Game|GetPlayerCharacter 1))
  ;[1 0.7647 0] Setting Camera As active camera
  (Game|Player|SetViewTargetwithBlend (Game|GetPlayerController 0) self 0.0 "VTBlend_Linear" 0.0 false))

(event EventTick
  (params (DeltaSeconds :type Float%20%28single-precision%29))
  (bind _player1 (Variables|Default|GetPlayer1))
  (bind _player2 (Variables|Default|GetPlayer2))
  (bind _returnvalue (Transformation|GetActorTransform _player2))
  (bind _returnvalue_2 (Transformation|GetActorTransform _player1))
  (bind _returnvalue_3 (+ (.z (.location _returnvalue_2)) (.z (.location _returnvalue))))
  (bind _returnvalue_4 (+ (.x (.location _returnvalue_2)) (.x (.location _returnvalue))))
  (bind _returnvalue_5 (+ (.y (.location _returnvalue_2)) (.y (.location _returnvalue))))
  (bind _returnvalue_6 (/ _returnvalue_3 2.0))
  (bind _returnvalue_7 (/ _returnvalue_5 2.0))
  (bind _returnvalue_8 (/ _returnvalue_4 2.0))
  (bind _returnvalue_9 (Math|Vector|MakeVector _returnvalue_8 _returnvalue_7 _returnvalue_6))
  ;[1 0.7647 0] Assiginig Camera to MidPointLocation
  (bind _output_get (Variables|Default|SetMidPointVector (Math|Vector|MakeVector (.x _returnvalue_9) (.y _returnvalue_9) (.z _returnvalue_9))))
  (Transformation|SetActorLocation (Variables|Default|GetMidPointVector) false false))

(fn ConstructionScript)